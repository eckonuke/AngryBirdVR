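; BP_Test_Building is a test building that reacts to being hit by a BP_Test_Bird.
; Its Box overlap passes the speed of the bird's Bird component to Damage, which increments DestroyState above a fixed velocity threshold.
; The following switch takes a constant 0 rather than DestroyState, so it always spawns an explosion emitter and never reaches the debug-print cases.
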(event OnComponentBeginOverlap(Box)
  (params (OverlappedComponent :type Primitive%20Component%20Object%20Reference) (OtherActor :type Actor%20Object%20Reference) (OtherComp :type Primitive%20Component%20Object%20Reference) (OtherBodyIndex :type Integer) (bFromSweep :type Boolean) (SweepResult :type Hit%20Result%20Structure%20%28by%20ref%29))
  (bind _asbp_test_bird (Utilities|Casting|CastToBP_Test_Bird OtherActor))
  (CallFunction|Damage (Math|Vector|VectorLength (Transformation|GetComponentVelocity (Variables|/Game/BluePrints/Test/BP_Test_Bird.BP_Test_Bird_C|GetBird _asbp_test_bird)))))

(event EventBeginPlay)

(event Collision|EventActorBeginOverlap
  (params (OtherActor :type Actor%20Object%20Reference)))

(event EventTick
  (params (DeltaSeconds :type Float%20%28single-precision%29)))

(fn ConstructionScript)

(fn Damage
  (params (incomingVelocity :type Float%20%28double-precision%29))
  (if (> incomingVelocity 1e+03)
    (Math|Integer|IncrementInt (Variables|Default|GetDestroyState)
      (:%20%20
        (switch int 0
          (:0
            (Effects|SpawnEmitteratLocation "/Game/StarterContent/Particles/P_Explosion.P_Explosion" "0, 0, 0" "0, 0, 0" "2.000000,2.000000,2.000000"))
          (:1
            (Development|PrintString "1"))
          (:2
            (Development|PrintString "2"))
          (:3
            (Development|PrintString "3")))))))