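; VR archery bow that a motion controller picks up, automatically spawning an arrow in the other hand and another after each shot.
; Near the notch the arrow hand eases into place; holding trigger draws along the arrow axis, clamped to a maximum, while aiming the bow hand along both hands.
; Releasing trigger fires with speed scaled by draw distance.
; Draw also drives ABP_Bow animation, haptics and audio.
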(event OnComponentBeginOverlap(Notch)
  (params (OverlappedComponent :type Primitive%20Component%20Object%20Reference) (OtherActor :type Actor%20Object%20Reference) (OtherComp :type Primitive%20Component%20Object%20Reference) (OtherBodyIndex :type Integer) (bFromSweep :type Boolean) (SweepResult :type Hit%20Result%20Structure%20%28by%20ref%29))
  ;[1 1 1] The hand holding the arrow is close to the buckle
  (if (and (Utilities|String|Contains (Utilities|GetDisplayName OverlappedComponent) "Con") (Utilities|IsValid (Variables|Default|GetHoldingArrowController)))
    (Actor|Tick|SetActorTickEnabled true)
    (Variables|Default|SetNotchTouching true)
    (Collision|SetCollisionEnabled (Variables|Default|GetNotch) "NoCollision")))

(event OnComponentEndOverlap(SkeletalMeshComponent)
  (params (OverlappedComponent :type Primitive%20Component%20Object%20Reference) (OtherActor :type Actor%20Object%20Reference) (OtherComp :type Primitive%20Component%20Object%20Reference) (OtherBodyIndex :type Integer))
  (Utilities|Casting|CastToBP_MotionController OtherActor)
  (CallFunction|SetBorderLine false))

(event OnComponentBeginOverlap(SkeletalMeshComponent)
  (params (OverlappedComponent :type Primitive%20Component%20Object%20Reference) (OtherActor :type Actor%20Object%20Reference) (OtherComp :type Primitive%20Component%20Object%20Reference) (OtherBodyIndex :type Integer) (bFromSweep :type Boolean) (SweepResult :type Hit%20Result%20Structure%20%28by%20ref%29))
  (if (Variables|Default|GetPickupable)
    (bind _asbp_motion_controller (Utilities|Casting|CastToBP_MotionController OtherActor))
    (Default|RumbleController _asbp_motion_controller 0.8)
    (CallFunction|SetBorderLine true)))

(event EventBeginPlay
  (Variables|Default|SetBowTransform (Transformation|GetWorldTransform (Variables|SkeletalMeshActor|GetSkeletalMeshComponent))))

(event Custom|DropArrow
  ;[1 1 1] Destroy Arrow
  (bind _holdingarrowcontroller (Variables|Default|GetHoldingArrowController)
    (:then
      (Variables|/Game/VR_Archery/Blueprint/BP_MotionController.BP_MotionController_C|SetBowArrowHolding _holdingarrowcontroller false)
      (Default|ReleaseActor (Variables|Default|GetHoldingArrowController))
      (Variables|Default|SetHoldingArrowController 0)
      (bind _arrowobject (Variables|Default|GetArrowObject)
        (:then
          (Actor|DestroyActor _arrowobject)
          (Variables|Default|SetArrowObject 0))
        (:else)))
    (:else)))

(event Custom|AutoGenerateArrow
  ;[1 1 1] Generate Arrow
  (bind _othercontroller (CallFunction|GetOtherHandController (Variables|Default|GetHoldingBowController)))
  (bind _output_get (Variables|Default|SetHoldingArrowController _othercontroller))
  (bind _returnvalue (Game|SpawnActorfromClass "/Game/VR_Archery/Blueprint/BowAndArrow/BP_Arrow.BP_Arrow_C" (Transformation|GetActorTransform _output_get) "Undefined" 0 0))
  (bind _output_get_2 (Variables|Default|SetArrowObject _returnvalue))
  (Variables|/Game/VR_Archery/Blueprint/BP_MotionController.BP_MotionController_C|SetAttachedActor (Variables|Default|GetHoldingArrowController) _output_get_2)
  (Class|BPIPickup|Pickup(Message) (Variables|Default|GetArrowObject) (Variables|Default|GetHoldingArrowController)))

(event EventPickup
  (params (MotionController :type BP%20Motion%20Controller%20Object%20Reference))
  ;[1 1 1] Bow Pickup
  (if (Variables|Default|GetPickupable)
    (Variables|Default|SetPickupable false)
    (Variables|Default|SetHoldingBowController MotionController)
    (Physics|SetSimulatePhysics (Variables|SkeletalMeshActor|GetSkeletalMeshComponent) false)
    (Collision|SetCollisionEnabled (Variables|SkeletalMeshActor|GetSkeletalMeshComponent) "NoCollision")
    (CallFunction|SetLineBow (Variables|Default|GetBowTransform))
    (Transformation|AttachComponentToComponent (Variables|SkeletalMeshActor|GetSkeletalMeshComponent) (Variables|/Game/VR_Archery/Blueprint/BP_MotionController.BP_MotionController_C|GetHandMesh (Variables|Default|GetHoldingBowController)) "Bow" "SnapToTarget" "SnapToTarget" "SnapToTarget" true)
    (CallFunction|SetBorderLine false)
    (Variables|/Game/VR_Archery/Blueprint/BP_MotionController.BP_MotionController_C|SetBowArrowHolding (Variables|Default|GetHoldingBowController) true)
    (CallFunction|SetHandAnimation (Variables|Default|GetHoldingBowAnim) (Variables|Default|GetHoldingBowController) 0.0)
    (CallFunction|AutoGenerateArrow)))

(event EventDrop
  ;[1 1 1] Bow Drop
  (Actor|DestroyActor (Variables|Default|GetLineBow))
  (Transformation|DetachFromActor "KeepWorld" "KeepWorld" "KeepWorld")
  (Transformation|SetWorldTransform (Variables|SkeletalMeshActor|GetSkeletalMeshComponent) (Variables|Default|GetBowTransform) false false)
  (Variables|Default|SetPickupable true)
  (Variables|/Game/VR_Archery/Blueprint/BP_MotionController.BP_MotionController_C|SetBowArrowHolding (Variables|Default|GetHoldingBowController) false)
  (Collision|SetCollisionEnabled (Variables|SkeletalMeshActor|GetSkeletalMeshComponent) "QueryOnly")
  (CallFunction|DropArrow))

(event Custom|PullTransition
  (bind _location (CallFunction|GetArrowHandProjectionVector))
  (bind _notch (Variables|Default|GetNotch))
  (bind _relativelocation (Variables|/Script/Engine.SceneComponent|GetRelativeLocation _notch))
  (bind _returnvalue (- _location _relativelocation))
  (bind _returnvalue_2 (Math|Vector|VectorLength _returnvalue))
  ;[1 1 1] Pull Bow
  (CallFunction|SetHandAnimation "NewEnumerator4" (Variables|Default|GetHoldingArrowController) 1.0)
  (CallFunction|SetHoldingBowHandTransform)
  (if (> (Math|Vector|DotProduct (Math|Vector|Normalize _returnvalue) (* (Math|Vector|GetRightVector (Variables|/Script/Engine.SceneComponent|GetRelativeRotation (Variables|SkeletalMeshActor|GetSkeletalMeshComponent))) -1.0)) 0.0)
    (Variables|Default|SetDistance _returnvalue_2)
    (if (< _returnvalue_2 (Variables|Default|GetMaxDestance))
      ;;[1 1 1] Set the arrow buckle, handle position and call the bow drawing animation
      (Transformation|SetRelativeLocation (Variables|Default|GetString) (CallFunction|GetArrowHandProjectionVector) false false)
      (Transformation|SetWorldLocation (Variables|/Game/VR_Archery/Blueprint/BP_MotionController.BP_MotionController_C|GetMotionController (Variables|Default|GetHoldingArrowController)) (Transformation|GetWorldLocation (Variables|Default|GetString)) false false)
      (CallFunction|SetBowAnimation (/ (Variables|Default|GetDistance) (Variables|Default|GetMaxDestance)))
      (Variables|Default|SetWillShoot true)
      (CallFunction|PullShock)
      (CallFunction|PullAudioPlay)
      (CallFunction|RemoveOutRangeShock)
      (else
        ;;[1 1 1] It is forbidden to pull beyond the maximum distance of the pantograph
        (Transformation|SetWorldLocation (Variables|/Game/VR_Archery/Blueprint/BP_MotionController.BP_MotionController_C|GetMotionController (Variables|Default|GetHoldingArrowController)) (Transformation|GetWorldLocation (Variables|Default|GetMaxLocation)) false false)
        (Variables|Default|SetDistance 49.0)
        (CallFunction|SetBowAnimation 1.0)
        (if (Variables|Default|GetOutOfRange)
          (CallFunction|PullAudioPlay)
          (else
            (Variables|Default|SetOutOfRange true)
            (CallFunction|BeginOutRangeShock)))))
    (else
      ;;[1 1 1] Reverse pantograph pulling is prohibited
      (Transformation|SetWorldLocation (Variables|/Game/VR_Archery/Blueprint/BP_MotionController.BP_MotionController_C|GetMotionController (Variables|Default|GetHoldingArrowController)) (Transformation|GetWorldLocation (Variables|Default|GetNotch)) false false)
      (CallFunction|PullAudioPlay))))

(event Custom|PullShock
  (bind _returnvalue (Game|GetPlayerController 0))
  (bind _location (CallFunction|GetArrowHandProjectionVector))
  (bind _distance (Variables|Default|GetDistance))
  (bind _maxdestance (Variables|Default|GetMaxDestance))
  (bind _notch (Variables|Default|GetNotch))
  (bind _returnvalue_2 (/ _distance _maxdestance))
  (bind _relativelocation (Variables|/Script/Engine.SceneComponent|GetRelativeLocation _notch))
  (bind _returnvalue_3 (- _location _relativelocation))
  (bind _returnvalue_4 (Math|Vector|VectorLength _returnvalue_3))
  ;[1 1 1] The handle shock when pulling the bow
  (if (>= (Math|Float|Absolute(Float) (- _returnvalue_4 (Variables|Default|GetLastShockDistance))) (Variables|Default|GetHapticDistanceThreshold))
    (Variables|Default|SetLastShockDistance (Math|Vector|VectorLength (- (CallFunction|GetArrowHandProjectionVector) (Variables|/Script/Engine.SceneComponent|GetRelativeLocation (Variables|Default|GetNotch)))))
    (if (< _returnvalue_4 (Variables|Default|GetMaxDestance))
      (Utilities|FlowControl|Sequence
        (:then_0
          (Class|PlayerController|PlayHapticEffect _returnvalue "/Game/VR_Archery/Curve/ECurve_HandShock.ECurve_HandShock" "Left" _returnvalue_2 false))
        (:then_1
          (Class|PlayerController|PlayHapticEffect _returnvalue "/Game/VR_Archery/Curve/ECurve_HandShock.ECurve_HandShock" "Right" _returnvalue_2 false))))))

(event Custom|ArrowNearBow
  (params (DetailTime :type Float%20%28double-precision%29))
  ;[1 1 1] The hand holding the arrow is close
  (if (and (Variables|Default|GetNotchTouching) (Utilities|IsValid (Variables|Default|GetHoldingArrowController)))
    (if (and (not (Variables|/Game/VR_Archery/Blueprint/BP_MotionController.BP_MotionController_C|GetTriggerClick (Variables|Default|GetHoldingArrowController))) (<= (CallFunction|GetDistanceFHandTNotch) 1e+01))
      (if (<= (CallFunction|GetDistanceFHandTNotch) 3.0)
        ;;[1 1 1] Set the transformation of the hand holding the bow to be consistent with that of the archer
        (Transformation|SetWorldRotation (Variables|/Game/VR_Archery/Blueprint/BP_MotionController.BP_MotionController_C|GetMotionController (Variables|Default|GetHoldingArrowController)) (Transformation|GetWorldRotation (Variables|/Game/VR_Archery/Blueprint/BP_MotionController.BP_MotionController_C|GetMotionController (Variables|Default|GetHoldingBowController))) false false)
        (Transformation|SetWorldLocation (Variables|/Game/VR_Archery/Blueprint/BP_MotionController.BP_MotionController_C|GetMotionController (Variables|Default|GetHoldingArrowController)) (Transformation|GetWorldLocation (Variables|Default|GetNotch)) false false)
        (CallFunction|SetHandAnimation "NewEnumerator4" (Variables|Default|GetHoldingArrowController) 1.0)
        (if (Variables|Default|GetAdsorbent)
          (Variables|Default|SetAdsorbent false)
          (Default|RumbleController (Variables|Default|GetHoldingArrowController) 0.8))
        (else
          ;;[1 1 1] Automatic adsorption of Archer
          (Transformation|SetWorldLocation (Variables|/Game/VR_Archery/Blueprint/BP_MotionController.BP_MotionController_C|GetMotionController (Variables|Default|GetHoldingArrowController)) (Math|Interpolation|VInterpTo (Transformation|GetWorldLocation (Variables|/Game/VR_Archery/Blueprint/BP_MotionController.BP_MotionController_C|GetMotionController (Variables|Default|GetHoldingArrowController))) (Transformation|GetWorldLocation (Variables|Default|GetNotch)) (stale EventTick DeltaSeconds) 5.0) false false)
          (Variables|Default|SetAdsorbent true)
          (CallFunction|SetHandAnimation "NewEnumerator4" (Variables|Default|GetHoldingArrowController) (/ (- 1e+01 (CallFunction|GetDistanceFHandTNotch)) 7.0))))
      (elif (not (Variables|Default|GetWillShoot))
        (CallFunction|SetHandAnimation "NewEnumerator4" (Variables|Default|GetHoldingArrowController) 0.0)))))

(event Custom|ShootEventListener
  ;[1 1 1] Bow pulling & archery monitoring
  (if (and (Variables|Default|GetNotchTouching) (Utilities|IsValid (Variables|Default|GetHoldingArrowController)))
    (if (Variables|/Game/VR_Archery/Blueprint/BP_MotionController.BP_MotionController_C|GetTriggerClick (Variables|Default|GetHoldingArrowController))
      (CallFunction|PullTransition)
      (elif (Variables|Default|GetWillShoot)
        (CallFunction|Shoot)
        (CallFunction|ShootShock)
        (CallFunction|RemoveOutRangeShock)
        (Variables|Default|SetWillShoot false)
        (Variables|Default|SetNotchTouching false)
        (Variables|Default|SetLastShockDistance 0.0)
        (CallFunction|PlayArrowReleaseAudio)))))

(event Custom|Shoot
  ;[1 1 1] Arrow shot
  (CallFunction|StopPullBackAudio)
  (Collision|SetCollisionEnabled (Variables|Default|GetNotch) "QueryOnly")
  (CallFunction|SetHoldingBowHandTransform)
  (if (< (Variables|Default|GetDistance) (Variables|Default|GetMaxDestance))
    ;;[1 1 1] Hold hand and bow and arrow transformation at the moment of arrow launch
    (Transformation|SetRelativeLocation (Variables|Default|GetString) (CallFunction|GetArrowHandProjectionVector) false false)
    (Transformation|SetWorldLocation (Variables|/Game/VR_Archery/Blueprint/BP_MotionController.BP_MotionController_C|GetMotionController (Variables|Default|GetHoldingArrowController)) (Transformation|GetWorldLocation (Variables|Default|GetString)) false false)
    (else
      (Transformation|SetWorldLocation (Variables|/Game/VR_Archery/Blueprint/BP_MotionController.BP_MotionController_C|GetMotionController (Variables|Default|GetHoldingArrowController)) (Transformation|GetWorldLocation (Variables|Default|GetMaxLocation)) false false)))
  (Class|BPIPickup|Drop(Message) (Variables|Default|GetArrowObject))
  (Default|Shoot (Variables|Default|GetArrowObject) (Math|Float|Lerp 0.0 3e+03 (/ (Variables|Default|GetDistance) (Variables|Default|GetMaxDestance))))
  ;;[1 1 1] Set the arrow buckle, handle position and call the bow drawing animation
  (Transformation|SetRelativeLocation (Variables|Default|GetString) (Transformation|GetWorldLocation (Variables|Default|GetNotch)) false false)
  (CallFunction|SetBowAnimation 0.0)
  ;;[1 1 1] Delete shot arrow Association
  (Variables|/Game/VR_Archery/Blueprint/BP_MotionController.BP_MotionController_C|SetAttachedActor (Variables|Default|GetHoldingArrowController) 0)
  (Variables|Default|SetHoldingArrowController 0)
  (Utilities|FlowControl|Delay 0.5)
  (Collision|SetCollisionEnabled (Variables|Default|GetNotch) "QueryOnly")
  (if (not (Variables|Default|GetPickupable))
    (CallFunction|AutoGenerateArrow)))

(event EventTick
  (params (DeltaSeconds :type Float%20%28single-precision%29))
  ;[1 1 1] Archery monitor
  (CallFunction|ShootEventListener)
  (CallFunction|ArrowNearBow 0.0))

(event Custom|PlayPullBackAudio
  (params (StartTime :type Float%20%28double-precision%29))
  (if (not (Audio|Components|Audio|IsPlaying (Variables|Default|GetPullBackAudio)))
    (Audio|Components|Audio|FadeIn (Variables|Default|GetPullBackAudio) 1.0 1.0 0.0 "Linear" :!class /Script/Engine.AudioComponent)))

(event Custom|StopPullBackAudio
  (if (Audio|Components|Audio|IsPlaying (Variables|Default|GetPullBackAudio))
    (Audio|Components|Audio|FadeOut (Variables|Default|GetPullBackAudio) 0.2 0.0 "Linear" :!class /Script/Engine.AudioComponent)))

(event Custom|PullAudioPlay
  (bind _location (CallFunction|GetArrowHandProjectionVector))
  (bind _notch (Variables|Default|GetNotch))
  (bind _relativelocation (Variables|/Script/Engine.SceneComponent|GetRelativeLocation _notch))
  (bind _returnvalue (- _location _relativelocation))
  (bind _returnvalue_2 (Math|Vector|VectorLength _returnvalue))
  ;[1 1 1] Bow pulling sound effect playback
  (Utilities|FlowControl|Sequence
    (:then_0
      (if (>= (Math|Float|Absolute(Float) (- _returnvalue_2 (Variables|Default|GetLastAudioDistance))) 0.2)
        (CallFunction|PlayPullBackAudio 0.0)
        (else
          (CallFunction|StopPullBackAudio))))
    (:then_1
      (Variables|Default|SetLastAudioDistance _returnvalue_2))))

(event Custom|PlayArrowReleaseAudio
  (bind _arrowobject (Variables|Default|GetArrowObject)
    (:then
      (Audio|Components|Audio|Play (Variables|/Game/VR_Archery/Blueprint/BowAndArrow/BP_Arrow.BP_Arrow_C|GetArrowReleaseAudio _arrowobject) 0.0))
    (:else)))

(fn ConstructionScript)

(fn SetBorderLine
  (params (ShowBorderLine :type Boolean))
  (Rendering|SetRenderCustomDepth (Variables|SkeletalMeshActor|GetSkeletalMeshComponent) ShowBorderLine))

(fn SetLineBow
  (params (Transform :type Transform))
  ;[1 1 1] Generate line bow
  (bind _returnvalue (Game|SpawnActorfromClass "/Game/VR_Archery/Blueprint/BowAndArrow/BP_LineBow.BP_LineBow_C" Transform "Undefined" 0 0))
  (bind _output_get (Variables|Default|SetLineBow _returnvalue))
  (Default|SetCollision _output_get))

(fn GetOtherHandController
  (params (HoldingController :type BP%20Motion%20Controller%20Object%20Reference))
  (bind _returnvalue (Game|Player|GetPlayerPawn 0))
  ;[1 1 1] Get another controller
  (if (Utilities|Enum|Equal(Enum) (Variables|/Game/VR_Archery/Blueprint/BP_MotionController.BP_MotionController_C|GetHand HoldingController) "Left")
    (bind _asbp_pawn (Utilities|Casting|CastToBP_Pawn _returnvalue))
    (return (Variables|/Game/VR_Archery/Blueprint/BP_Pawn.BP_Pawn_C|GetRightController _asbp_pawn))
    (else
      (bind _asbp_pawn_2 (Utilities|Casting|CastToBP_Pawn _returnvalue))
      (return (Variables|/Game/VR_Archery/Blueprint/BP_Pawn.BP_Pawn_C|GetLeftController _asbp_pawn_2)))))

(fn SetBowAnimation
  (params (Distance :type Float%20%28double-precision%29))
  ;[1 1 1] Animate bow
  (bind _asabp_bow (Utilities|Casting|CastToABP_Bow (Components|SkeletalMesh|GetAnimInstance (Variables|SkeletalMeshActor|GetSkeletalMeshComponent))))
  (Variables|/Game/VR_Archery/Animations/Bow/ABP_Bow.ABP_Bow_C|SetDistance _asabp_bow Distance))

(fn SetHoldingBowHandTransform
  (bind _holdingbowcontroller (Variables|Default|GetHoldingBowController))
  (bind _holdingarrowcontroller (Variables|Default|GetHoldingArrowController))
  (bind _motioncontroller (Variables|/Game/VR_Archery/Blueprint/BP_MotionController.BP_MotionController_C|GetMotionController _holdingbowcontroller))
  (bind _motioncontroller_2 (Variables|/Game/VR_Archery/Blueprint/BP_MotionController.BP_MotionController_C|GetMotionController _holdingarrowcontroller))
  (bind _returnvalue (Transformation|GetWorldLocation _motioncontroller))
  (bind _returnvalue_2 (Transformation|GetWorldLocation _motioncontroller_2))
  (bind _returnvalue_3 (Math|Rotator|FindLookatRotation _returnvalue_2 _returnvalue))
  (bind (_roll _pitch _yaw) (Math|Rotator|BreakRotator _returnvalue_3))
  ;[1 1 1] Set the world transformation of the hand holding the bow
  (Transformation|SetWorldRotation (Variables|/Game/VR_Archery/Blueprint/BP_MotionController.BP_MotionController_C|GetMotionController (Variables|Default|GetHoldingBowController)) (Math|Rotator|MakeRotator (.Roll (Math|Rotator|BreakRotator (Variables|/Script/Engine.SceneComponent|GetRelativeRotation (Variables|/Game/VR_Archery/Blueprint/BP_MotionController.BP_MotionController_C|GetMotionController (Variables|Default|GetHoldingBowController))))) _pitch _yaw) false false)
  ;[1 1 1] Set the transformation of the hand holding the bow to be consistent with that of the hand holding the arrow
  (Transformation|SetWorldRotation (Variables|/Game/VR_Archery/Blueprint/BP_MotionController.BP_MotionController_C|GetMotionController (Variables|Default|GetHoldingArrowController)) (Transformation|GetWorldRotation (Variables|/Game/VR_Archery/Blueprint/BP_MotionController.BP_MotionController_C|GetMotionController (Variables|Default|GetHoldingBowController))) false false))

(fn GetArrowHandProjectionVector
  (return (Math|Vector|ProjectVectorontoVector (Math|Transform|InverseTransformLocation (Transformation|GetActorTransform) (Transformation|GetWorldLocation (Variables|/Game/VR_Archery/Blueprint/BP_MotionController.BP_MotionController_C|GetMotionController (Variables|Default|GetHoldingArrowController)))) (* (Math|Vector|GetRightVector (Variables|/Script/Engine.SceneComponent|GetRelativeRotation (Variables|SkeletalMeshActor|GetSkeletalMeshComponent))) -1.0))))

(fn GetDistanceFHandTNotch
  ;[1 1 1] Bow distance
  (return (Math|Vector|Distance(Vector) (Transformation|GetWorldLocation (Variables|/Game/VR_Archery/Blueprint/BP_MotionController.BP_MotionController_C|GetMotionController (Variables|Default|GetHoldingArrowController))) (Transformation|GetWorldLocation (Variables|Default|GetNotch)))))

(fn OutOfRangeShock
  (Class|PlayerController|PlayHapticEffect (Game|GetPlayerController 0) "/Game/VR_Archery/Curve/ECurve_OutRange.ECurve_OutRange" (Variables|/Game/VR_Archery/Blueprint/BP_MotionController.BP_MotionController_C|GetHand (Variables|Default|GetHoldingArrowController)) 1.0 false))

(fn BeginOutRangeShock
  (bind _returnvalue (Utilities|Time|SetTimerbyFunctionName 0 "OutOfRangeShock" 0.5 true))
  (Variables|Default|SetTimer _returnvalue))

(fn RemoveOutRangeShock
  (Utilities|Time|ClearTimerbyFunctionName 0 "OutOfRangeShock")
  (Variables|Default|SetOutOfRange false))

(fn ShootShock
  (Class|PlayerController|PlayHapticEffect (Game|GetPlayerController 0) "/Game/VR_Archery/Curve/ECurve_Shoot.ECurve_Shoot" (Variables|/Game/VR_Archery/Blueprint/BP_MotionController.BP_MotionController_C|GetHand (Variables|Default|GetHoldingBowController)) 1.0 false))