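; BP_Arrow is the VR archery arrow that a motion controller picks up and that flies as a projectile when shot.
; Pickup runs once, disabling physics, snapping the mesh to the hand's Arrow socket and updating the controller's holding flag and hand animation, while Drop only detaches it.
; Shoot launches ProjectileMovement at the given velocity and enables the ArrowBox overlap query.
; The first non-MotionController overlap stops the arrow, which is destroyed after a delay.
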(event OnComponentBeginOverlap(ArrowBox)
  (params (OverlappedComponent :type Primitive%20Component%20Object%20Reference) (OtherActor :type Actor%20Object%20Reference) (OtherComp :type Primitive%20Component%20Object%20Reference) (OtherBodyIndex :type Integer) (bFromSweep :type Boolean) (SweepResult :type Hit%20Result%20Structure%20%28by%20ref%29))
  (bind _projectilemovement (Variables|Default|GetProjectileMovement))
  (if (and (Variables|Default|GetIsShoot) (not (Utilities|String|Contains (Utilities|GetDisplayName OtherComp) "MotionController")))
    (Utilities|FlowControl|DoOnce false
      (:Completed
        (Components|Movement|StopMovementImmediately _projectilemovement)
        (Components|Activation|SetActive _projectilemovement false false)
        (Utilities|FlowControl|Delay 5.0)
        (Actor|DestroyActor)))))

(event Custom|Shoot
  (params (Velocity :type Float%20%28double-precision%29))
  (bind _projectilemovement (Variables|Default|GetProjectileMovement))
  (bind _output_get (Variables|/Script/Engine.ProjectileMovementComponent|SetInitialSpeed _projectilemovement Velocity))
  (bind _output_get_2 (Variables|/Script/Engine.ProjectileMovementComponent|SetMaxSpeed _projectilemovement _output_get))
  (Game|Components|ProjectileMovement|SetVelocityinLocalSpace (Variables|Default|GetProjectileMovement) (Math|Vector|MakeVector _output_get_2 0.0 0.0))
  (Variables|Default|SetIsShoot true)
  (Variables|/Script/Engine.ProjectileMovementComponent|SetbRotationFollowsVelocity (Variables|Default|GetProjectileMovement) true)
  (Components|Activation|SetActive (Variables|Default|GetProjectileMovement) true false)
  (Collision|SetCollisionEnabled (Variables|Default|GetArrowBox) "QueryOnly"))

(event EventPickup
  (params (MotionController :type BP%20Motion%20Controller%20Object%20Reference))
  (if (not (Variables|Default|GetPickupable))
    (Variables|Default|SetPickupable true)
    (Variables|Default|SetHoldingController MotionController)
    (Physics|SetSimulatePhysics (Variables|Debug|GetStaticMeshComponent) false)
    (Transformation|AttachComponentToComponent (Variables|Debug|GetStaticMeshComponent) (Variables|/Game/VR_Archery/Blueprint/BP_MotionController.BP_MotionController_C|GetHandMesh (Variables|Default|GetHoldingController)) "Arrow" "SnapToTarget" "SnapToTarget" "SnapToTarget" false)
    (Variables|/Game/VR_Archery/Blueprint/BP_MotionController.BP_MotionController_C|SetBowArrowHolding (Variables|Default|GetHoldingController) true)
    (CallFunction|SetHandAnimation (Variables|Default|GetHandAnimation) (Variables|Default|GetHoldingController) 0.0)))

(event EventDrop
  (Transformation|DetachFromActor "KeepWorld" "KeepWorld" "KeepWorld"))

(fn ConstructionScript)