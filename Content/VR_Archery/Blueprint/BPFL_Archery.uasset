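; Blueprint function library for the VR archery module that drives hand animations on the controllers.
; SetHandAnimation takes a holding controller, casts its hand mesh anim instance to ABP_Hand, and writes the grip state and arrow-hand-to-notch distance into it.
; The animation blueprint uses those values to pose the hand.
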(fn SetHandAnimation
  (params (HandAnimation :type E_GripEnum%20Enum :default "NewEnumerator0") (HoldingController :type BP%20Motion%20Controller%20Object%20Reference) (ArrowHandToNotch :type Float%20%28single-precision%29))
  (LocalVariables|SetAnimation HandAnimation)
  (LocalVariables|SetController HoldingController)
  (LocalVariables|SetDistance ArrowHandToNotch)
  (bind _asabp_hand (Utilities|Casting|CastToABP_Hand (Components|SkeletalMesh|GetAnimInstance (Variables|/Game/VR_Archery/Blueprint/BP_MotionController.BP_MotionController_C|GetHandMesh (LocalVariables|GetController)))))
  (Variables|/Game/VR_Archery/Animations/Hand/ABP_Hand.ABP_Hand_C|SetGripState _asabp_hand (LocalVariables|GetAnimation))
  (Variables|/Game/VR_Archery/Animations/Hand/ABP_Hand.ABP_Hand_C|SetArrowHandToNotch _asabp_hand (LocalVariables|GetDistance)))